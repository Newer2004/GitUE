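; Leon is a playable third-person character with free-roam and aim camera modes, driven by Enhanced Input.
; Look input turns controller yaw but applies pitch directly to the spring arm within clamped limits, while movement follows control rotation.
; Aiming swaps spring arm length and offset and switches from movement-oriented to controller-facing rotation after short delays.
; Sprint raises walk speed unless aiming is already active when it starts.
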(event `self.ReceiveBeginPlay`
  (bind _springarm (`self.SpringArm`))
  (`EnhancedInputSubsystemInterface.AddMappingContext` (pcsubsystem `EnhancedInputLocalPlayerSubsystem` (`GameplayStatics.GetPlayerController` 0)) "/Game/Game/Leon/Input/IMC_Leon.IMC_Leon" 0 (struct))
  (set `SpringArmComponent.TargetArmLength` (`self.FreeModeTargetArmLength`) _springarm)
  (set `SpringArmComponent.SocketOffset` (`self.FreeModeSocketOffset`) _springarm))

(event `EnhancedInput|/Game/Game/Leon/Input/IA_RotateCamera`
  (params (ActionValue :type "Vector2D Structure") (ElapsedSeconds :type "Float (double-precision)") (TriggeredSeconds :type "Float (double-precision)") (InputAction :type "InputAction Object Reference" :default "/Game/Game/Leon/Input/IA_RotateCamera.IA_RotateCamera"))
  (bind (_x _y) (`KismetMathLibrary.BreakVector2D` ActionValue))
  (bind (_relativerotation_roll _relativerotation_pitch _relativerotation_yaw) (`KismetMathLibrary.BreakRotator` (`SceneComponent.RelativeRotation` (`self.SpringArm`))))
  (:`Triggered`
    (`self.AddControllerYawInput` _x)
    (set `self.VerticalAngle` (`KismetMathLibrary.ClampAngle` (+ _y (`self.VerticalAngle`)) -80.0 60.0))
    (`SceneComponent.K2_SetRelativeRotation` (`self.SpringArm`) (`KismetMathLibrary.MakeRotator` 0.0 (`self.VerticalAngle`) _relativerotation_yaw) false false)))

(event `EnhancedInput|/Game/Game/Leon/Input/IA_Move`
  (params (ActionValue :type "Vector2D Structure") (ElapsedSeconds :type "Float (double-precision)") (TriggeredSeconds :type "Float (double-precision)") (InputAction :type "InputAction Object Reference" :default "/Game/Game/Leon/Input/IA_Move.IA_Move"))
  (bind (_x _y) (`KismetMathLibrary.BreakVector2D` ActionValue))
  (bind _returnvalue (`self.GetControlRotation`))
  (:`Triggered`
    (`self.AddMovementInput` (+ (* _x (`KismetMathLibrary.GetForwardVector` _returnvalue)) (* _y (`KismetMathLibrary.GetRightVector` _returnvalue))))))

(event `EnhancedInput|/Game/Game/Leon/Input/IA_Sprinting`
  (params (ActionValue :type Boolean) (ElapsedSeconds :type "Float (double-precision)") (TriggeredSeconds :type "Float (double-precision)") (InputAction :type "InputAction Object Reference" :default "/Game/Game/Leon/Input/IA_Sprinting.IA_Sprinting"))
  (bind _charactermovement (`self.CharacterMovement`))
  (:`Started`
    (if (not (`self.IsAiming`))
      (set `CharacterMovementComponent.MaxWalkSpeed` 300.0 _charactermovement)))
  (:`Completed`
    (set `CharacterMovementComponent.MaxWalkSpeed` 120.0 _charactermovement)))

(event `EnhancedInput|/Game/Game/Leon/Input/IA_Aim`
  (params (ActionValue :type Boolean) (ElapsedSeconds :type "Float (double-precision)") (TriggeredSeconds :type "Float (double-precision)") (InputAction :type "InputAction Object Reference" :default "/Game/Game/Leon/Input/IA_Aim.IA_Aim"))
  (bind _charactermovement (`self.CharacterMovement`))
  (bind _springarm (`self.SpringArm`))
  (bind _charactermovement_2 (`self.CharacterMovement`))
  (bind _springarm_2 (`self.SpringArm`))
  (:`Started`
    (set `self.IsAiming` true)
    (`KismetSystemLibrary.Delay` 0.7)
    (set `CharacterMovementComponent.bUseControllerDesiredRotation` true _charactermovement)
    (set `CharacterMovementComponent.bOrientRotationToMovement` false _charactermovement)
    (set `SpringArmComponent.TargetArmLength` (`self.AimModeTargetArmLength`) _springarm_2)
    (set `SpringArmComponent.SocketOffset` (`self.AimModeSocketOffset`) _springarm_2))
  (:`Completed`
    (set `self.IsAiming` false)
    (`KismetSystemLibrary.Delay` 0.6)
    (set `CharacterMovementComponent.bOrientRotationToMovement` true _charactermovement_2)
    (set `CharacterMovementComponent.bUseControllerDesiredRotation` false _charactermovement_2)
    (set `SpringArmComponent.TargetArmLength` (`self.FreeModeTargetArmLength`) _springarm)
    (set `SpringArmComponent.SocketOffset` (`self.FreeModeSocketOffset`) _springarm)))

(fn `UserConstructionScript`)