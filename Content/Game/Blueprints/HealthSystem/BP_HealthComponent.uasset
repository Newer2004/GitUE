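; BP_HealthComponent tracks Health against MaxHealth and exposes Hurt and Heal functions to change it.
; Hurt sets Health to Damage minus Health (operands reversed from a usual subtraction), clamped to the valid range, and returns whether it reached zero.
; Heal returns false at full health, otherwise adds the amount with clamping, prints the new value and returns true.
; BeginPlay and Tick are unused.
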(fn `Heal`
  (params (Amount :type Integer))
  (returns (Healed :type Boolean))
  (if (== (`self.Health`) (`self.Max Health`))
    (return false)
    (else
      (bind _output_get (set `self.Health` (`KismetMathLibrary.Clamp` (+ Amount (`self.Health`)) 0 (`self.Max Health`))))
      (`KismetSystemLibrary.PrintString` (`KismetStringLibrary.Conv_IntToString` _output_get))
      (return true))))

(fn `Hurt`
  (params (Damage :type Integer))
  (returns (Dead :type Boolean))
  (bind _output_get (set `self.Health` (`KismetMathLibrary.Clamp` (- Damage (`self.Health`)) 0 (`self.Max Health`))))
  (return (<= _output_get 0)))