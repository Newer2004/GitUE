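; BP_Window is an interactable window the player can look out of and back from.
; Interact toggles IsLooking, blending the view target between the window actor and the player character while hiding the character.
; Input moves between character and window, so the window's own IA_Interact binding can exit the view.
; The interaction prompt switches between "Look" and "Back" to match the state.
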(event `self.Interact`
  (bind _returnvalue (`GameplayStatics.GetPlayerCharacter` 0))
  (bind _returnvalue_2 (`GameplayStatics.GetPlayerController` 0))
  (bind _returnvalue_3 (`GameplayStatics.GetPlayerCharacter` 0))
  (if (`self.Is Looking`)
    (set `self.Is Looking` false)
    (`self.EnableInput` _returnvalue_3 _returnvalue_2)
    (`self.SetActorHiddenInGame` _returnvalue_3 false)
    (`self.DisableInput` self (`GameplayStatics.GetPlayerController` 0))
    (`PlayerController.SetViewTargetWithBlend` (`GameplayStatics.GetPlayerController` 0) (`GameplayStatics.GetPlayerCharacter` 0) 0.5 "VTBlend_Linear" 0.0 false)
    (`self.Set Prompt Description` "Look")
    (else
      (set `self.Is Looking` true)
      (`self.DisableInput` _returnvalue _returnvalue_2)
      (`self.SetActorHiddenInGame` _returnvalue true)
      (`self.EnableInput` self (`GameplayStatics.GetPlayerController` 0))
      (`PlayerController.SetViewTargetWithBlend` (`GameplayStatics.GetPlayerController` 0) self 0.5 "VTBlend_Linear" 0.0 false)
      (`self.Set Prompt Description` "Back"))))

(event `EnhancedInput|/Game/Game/Leon/Input/IA_Interact`
  (params (ActionValue :type Boolean) (ElapsedSeconds :type "Float (double-precision)") (TriggeredSeconds :type "Float (double-precision)") (InputAction :type "InputAction Object Reference" :default "/Game/Game/Leon/Input/IA_Interact.IA_Interact"))
  (:`Started`
    (`self.Interact`)))

(fn `UserConstructionScript`
  (`parent.UserConstructionScript`))