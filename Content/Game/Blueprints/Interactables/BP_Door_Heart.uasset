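; BP_Door_Heart is an interactable door that toggles open and closed with a timeline-driven yaw swing, updating its prompt text.
; When locked, it requires and consumes a named key from BP_Leon's inventory.
; Unlocking switches view to the door, hides the player and disables their input while a timeline animates the key.
; The door opens after a fixed delay, separate from the key timeline's finish, which restores player view and control.
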(event `self.Interact`
  (if (`self.Is Locked`)
    (bind _was_unlock (`self.Open Locked Door`))
    (if _was_unlock
      (`self.Animation Unlock Door`)
      (`KismetSystemLibrary.Delay` 4.0)
      (if (`self.Is Closed`) :!label _label
        (set `self.Is Closed` false)
        (`self.Set Prompt Description` "Close")
        (bind (_direction _float) (`Timeline|Timeline` :!label _label_2)
          (:`Update`
            (`SceneComponent.K2_SetRelativeRotation` (`self.SM_Door`) (`KismetMathLibrary.MakeRotator` 0.0 0.0 (`KismetMathLibrary.Lerp` 0.0 90.0 _float)) false false)))
        (else
          (set `self.Is Closed` true)
          (`self.Set Prompt Description` "Open")
          (goto _label_2 :!via `Reverse`))))
    (else
      (goto _label))))

(event `self.ReceiveBeginPlay`
  (`parent.ReceiveBeginPlay`))

(event `Animation Unlock Door`
  (bind _centerspecial (`self.CenterSpecial`))
  (bind _centerspecial_2 (`self.CenterSpecial`))
  (bind (_relativerotation_roll _relativerotation_pitch _relativerotation_yaw) (`KismetMathLibrary.BreakRotator` (`SceneComponent.RelativeRotation` _centerspecial_2)))
  (bind (_relativelocation_x _relativelocation_y _relativelocation_z) (`KismetMathLibrary.BreakVector` (`SceneComponent.RelativeLocation` _centerspecial_2)))
  (`self.Change Camera`)
  (`SceneComponent.SetHiddenInGame` (`self.Key`) false false)
  (bind (_direction _float_vector _float_rotate) (`Timeline|Key Timeline`)
    (:`Update`
      (`SceneComponent.K2_SetRelativeLocation` _centerspecial (`KismetMathLibrary.MakeVector` (`KismetMathLibrary.Lerp` _relativelocation_x -8.0 _float_vector) _relativelocation_y _relativelocation_z) false false)
      (`SceneComponent.K2_SetRelativeRotation` _centerspecial (`KismetMathLibrary.MakeRotator` (`KismetMathLibrary.Lerp` 0.0 90.0 _float_rotate) _relativerotation_pitch _relativerotation_yaw) false false))
    (:`Finished`
      (`SceneComponent.SetHiddenInGame` (`self.Key`) true false)
      (set `self.Is Locked` false)
      (`self.Change Camera`))))

(fn `Change Camera`
  (bind _returnvalue (`GameplayStatics.GetPlayerController` 0))
  (bind _returnvalue_2 (`GameplayStatics.GetPlayerCharacter` 0))
  (bind _returnvalue_3 (`GameplayStatics.GetPlayerController` 0))
  (if (`self.Is Looking`)
    (set `self.Is Looking` false)
    (`SceneComponent.SetHiddenInGame` (`self.Prompt`) false false)
    (`self.EnableInput` _returnvalue_2 _returnvalue)
    (`self.SetActorHiddenInGame` _returnvalue_2 false)
    (`self.DisableInput` self _returnvalue_3)
    (`PlayerController.SetViewTargetWithBlend` (`GameplayStatics.GetPlayerController` 0) (`GameplayStatics.GetPlayerCharacter` 0) 0.0 "VTBlend_Linear" 0.0 false)
    (else
      (set `self.Is Looking` true)
      (`SceneComponent.SetHiddenInGame` (`self.Prompt`) true false)
      (`self.DisableInput` _returnvalue_2 _returnvalue)
      (`self.SetActorHiddenInGame` _returnvalue_2 true)
      (`self.EnableInput` self _returnvalue_3)
      (`PlayerController.SetViewTargetWithBlend` (`GameplayStatics.GetPlayerController` 0) self 0.0 "VTBlend_Linear" 0.0 false))))

(fn `Open Locked Door`
  (returns (`Was Unlock` :type Boolean))
  (bind _asbp_leon (cast `/Game/Game/Leon/Blueprint/BP_Leon` (`GameplayStatics.GetPlayerCharacter` 0)))
  (bind _inventory (`/Game/Game/Leon/Blueprint/BP_Leon.Inventory` _asbp_leon))
  (bind _item (`/Game/Game/Blueprints/InventorySystem/UI_InventoryMenu.Find Slot by Name` _inventory (`self.Key Name`)))
  (if (`KismetTextLibrary.EqualEqual_TextText` "" (break `/Game/Game/Blueprints/InventorySystem/STRUCT_Item` _item))
    (`KismetSystemLibrary.PrintString` (`KismetTextLibrary.Conv_TextToString` (`self.Key Name`)))
    (return false)
    (else
      (`/Game/Game/Blueprints/InventorySystem/UI_InventoryMenu.Clear Slot by Name` _inventory (`self.Key Name`))
      (return true))))

(fn `UserConstructionScript`
  (`parent.UserConstructionScript`))