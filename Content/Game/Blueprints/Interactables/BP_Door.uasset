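; Interactable door that toggles open and closed on Interact and switches its prompt between "Open" and "Close".
; A Timeline drives the door mesh's yaw through a 90-degree swing, playing to open and reversing to close, with IsClosed tracking the state.
; OpenLockedDoor is an unfinished stub: it casts the player to BP_Leon but does nothing with the Inventory it references.
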(event `self.Interact`
  (if (`self.Is Closed`)
    (set `self.Is Closed` false)
    (`self.Set Prompt Description` "Close")
    (bind (_direction _float) (`Timeline|Timeline` :!label _label)
      (:`Update`
        (`SceneComponent.K2_SetRelativeRotation` (`self.SM_Door`) (`KismetMathLibrary.MakeRotator` 0.0 0.0 (`KismetMathLibrary.Lerp` 0.0 90.0 _float)) false false)))
    (else
      (set `self.Is Closed` true)
      (`self.Set Prompt Description` "Open")
      (goto _label :!via `Reverse`))))

(fn `Open Locked Door`
  (bind _asbp_leon (cast `/Game/Game/Leon/Blueprint/BP_Leon` (`GameplayStatics.GetPlayerCharacter` 0))))

(fn `UserConstructionScript`
  (`parent.UserConstructionScript`))