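; BP_Safe is an interactable safe with a numpad interface that yields a medallion when opened.
; Interact shows UI_Numpad with the mouse cursor and pauses the game, while Leave restores game-only input and unpauses.
; Open unpauses, spawns BP_Medallion2 at Area and plays a timeline that swings SafeDoor open by yaw.
; That timeline's update also restores game input and disables InteractionTrigger collision.
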(event `self.Interact`
  (bind _returnvalue (`GameplayStatics.GetPlayerController` 0))
  (bind _returnvalue_2 (`|CreateWidget` "/Game/Game/Blueprints/Interactables/Safe/UI_Numpad.UI_Numpad_C"))
  (`UserWidget.AddToViewport` _returnvalue_2 0)
  (`WidgetBlueprintLibrary.SetInputMode_GameAndUIEx` _returnvalue _returnvalue_2)
  (set `PlayerController.bShowMouseCursor` true _returnvalue)
  (`GameplayStatics.SetGamePaused` true))

(event `Open`
  (`GameplayStatics.SetGamePaused` false)
  (`|SpawnActorFromClass` "/Game/Game/Blueprints/Interactables/Pickup/BP_Medallion2.BP_Medallion2_C" (`self.Area`) "Undefined" "MultiplyWithRoot" null null)
  (bind (_direction _float) (`Timeline|Timeline`)
    (:`Update`
      (`SceneComponent.K2_SetRelativeRotation` (`self.Safe_Door`) (`KismetMathLibrary.MakeRotator` 0.0 0.0 (`KismetMathLibrary.Lerp` 0.0 -90.0 _float)) false false)
      (set `PlayerController.bShowMouseCursor` false (`GameplayStatics.GetPlayerController` 0))
      (`WidgetBlueprintLibrary.SetInputMode_GameOnly` (`GameplayStatics.GetPlayerController` 0))
      (`PrimitiveComponent.SetCollisionEnabled` (`self.Interaction Trigger`) "NoCollision"))))

(event `Leave`
  (set `PlayerController.bShowMouseCursor` false (`GameplayStatics.GetPlayerController` 0))
  (`WidgetBlueprintLibrary.SetInputMode_GameOnly` (`GameplayStatics.GetPlayerController` 0))
  (`GameplayStatics.SetGamePaused` false))

(fn `UserConstructionScript`
  (`parent.UserConstructionScript`))