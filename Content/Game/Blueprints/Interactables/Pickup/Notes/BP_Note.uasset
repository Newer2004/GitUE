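; BP_Note is an interactable note pickup that the player opens to read and closes again.
; Interact toggles a reading state that creates a widget on screen, freezes the game through zero global time dilation, shows the cursor and switches to game-and-UI input.
; A second Interact or a StopReading call shares one close path that removes the widget and restores time, cursor and game-only input.
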(event `/Game/Game/Blueprints/Interactables/BP_Interactable_Base.Interact`
  (bind _returnvalue (`GameplayStatics.GetPlayerController` 0))
  (bind _returnvalue_2 (`GameplayStatics.GetPlayerController` 0))
  (if (`self.Is Reading`)
    (set `self.Is Reading` false :!label _label)
    (`GameplayStatics.SetGlobalTimeDilation` 1.0)
    (set `PlayerController.bShowMouseCursor` false _returnvalue)
    (`WidgetBlueprintLibrary.SetInputMode_GameOnly` _returnvalue)
    (`Widget.RemoveFromParent` (stale _returnvalue_3))
    (else
      (set `self.Is Reading` true)
      (`GameplayStatics.SetGlobalTimeDilation` 0.0)
      (set `PlayerController.bShowMouseCursor` true _returnvalue_2)
      (bind _returnvalue_3 (`|CreateWidget` (`self.Class_0`)))
      (`WidgetBlueprintLibrary.SetInputMode_GameAndUIEx` _returnvalue_2 _returnvalue_3)
      (`UserWidget.AddToViewport` _returnvalue_3 0))))

(event `Stop Reading`
  (goto _label))

(fn `UserConstructionScript`
  (`parent.UserConstructionScript`))