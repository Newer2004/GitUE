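; BP_Interactable_Base is the base Blueprint for interactable objects, providing a widget prompt that describes the available action.
; On BeginPlay it passes ActionDescription to the UI_Prompt widget held by the Prompt component.
; ShowPrompt toggles that component's visibility.
; The Interact event is a fallback that prints a warning naming the object when interaction is not set up.
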(event `self.ReceiveBeginPlay`
  (`self.Set Prompt Description` (`self.Action Description`)))

(event `Interact`
  (`KismetSystemLibrary.PrintString` (`KismetStringLibrary.Concat_StrStr` "Interaction not set up on" (`KismetSystemLibrary.GetDisplayName` self))))

(fn `Set Prompt Description`
  (params (Description :type Text))
  (bind _asui_prompt (cast `/Game/Game/Blueprints/Interactables/UI_Prompt` (`WidgetComponent.GetWidget` (`self.Prompt`))))
  (`/Game/Game/Blueprints/Interactables/UI_Prompt.Set Description` _asui_prompt Description))

(fn `Show Prompt`
  (params (Show :type Boolean))
  (`SceneComponent.SetHiddenInGame` (`self.Prompt`) (not Show) false))

(fn `UserConstructionScript`)