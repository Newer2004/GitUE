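; BP_Statue is an interactable puzzle statue that takes three medallions from the player's inventory and moves its mesh once they are placed.
; On Interact, three functions each look up a medallion in BP_Leon's inventory, clear its slot and reveal the matching mesh, or print the missing name.
; Only when all three succeed in one interaction does a Timeline lerp the mesh's Z and disable the interaction trigger's collision.
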(event `self.Interact`
  (bind _staticmesh (`self.StaticMesh`))
  (bind (_relativelocation_x _relativelocation_y _relativelocation_z) (`KismetMathLibrary.BreakVector` (`SceneComponent.RelativeLocation` _staticmesh)))
  (if (not (`self.Is Open`))
    (bind _m1_done (`self.Put Medallion 1`))
    (bind _m2_done (`self.Put Medallion 2`))
    (bind _m3_done (`self.Put Medallion 3`))
    (if (and _m3_done (and _m2_done _m1_done))
      (bind (_direction _float) (`Timeline|Timeline`)
        (:`Update`
          (`SceneComponent.K2_SetRelativeLocation` _staticmesh (`KismetMathLibrary.MakeVector` _relativelocation_x _relativelocation_y (`KismetMathLibrary.Lerp` _relativelocation_z (- (`self.Upp`) (`self.Downn`)) _float)) false false)
          (`PrimitiveComponent.SetCollisionEnabled` (`self.Interaction Trigger`) "NoCollision"))))))

(fn `Put Medallion 1`
  (returns (M1_done :type Boolean))
  (bind _asbp_leon (cast `/Game/Game/Leon/Blueprint/BP_Leon` (`GameplayStatics.GetPlayerCharacter` 0)))
  (bind _inventory (`/Game/Game/Leon/Blueprint/BP_Leon.Inventory` _asbp_leon))
  (bind _item (`/Game/Game/Blueprints/InventorySystem/UI_InventoryMenu.Find Slot by Name` _inventory (`self.Medallion 1`)))
  (if (`KismetTextLibrary.EqualEqual_TextText` "" (break `/Game/Game/Blueprints/InventorySystem/STRUCT_Item` _item))
    (`KismetSystemLibrary.PrintString` (`KismetTextLibrary.Conv_TextToString` (`self.Medallion 1`)))
    (else
      (`/Game/Game/Blueprints/InventorySystem/UI_InventoryMenu.Clear Slot by Name` _inventory (`self.Medallion 1`))
      (`SceneComponent.SetHiddenInGame` (`self.medal1`) false false)
      (return true))))

(fn `Put Medallion 2`
  (returns (`M2 done` :type Boolean))
  (bind _asbp_leon (cast `/Game/Game/Leon/Blueprint/BP_Leon` (`GameplayStatics.GetPlayerCharacter` 0)))
  (bind _inventory (`/Game/Game/Leon/Blueprint/BP_Leon.Inventory` _asbp_leon))
  (bind _item (`/Game/Game/Blueprints/InventorySystem/UI_InventoryMenu.Find Slot by Name` _inventory (`self.Medallion 2`)))
  (if (`KismetTextLibrary.EqualEqual_TextText` "" (break `/Game/Game/Blueprints/InventorySystem/STRUCT_Item` _item))
    (`KismetSystemLibrary.PrintString` (`KismetTextLibrary.Conv_TextToString` (`self.Medallion 2`)))
    (else
      (`/Game/Game/Blueprints/InventorySystem/UI_InventoryMenu.Clear Slot by Name` _inventory (`self.Medallion 2`))
      (`SceneComponent.SetHiddenInGame` (`self.medal2`) false false)
      (return true))))

(fn `Put Medallion 3`
  (returns (`M3 Done` :type Boolean))
  (bind _asbp_leon (cast `/Game/Game/Leon/Blueprint/BP_Leon` (`GameplayStatics.GetPlayerCharacter` 0)))
  (bind _inventory (`/Game/Game/Leon/Blueprint/BP_Leon.Inventory` _asbp_leon))
  (bind _item (`/Game/Game/Blueprints/InventorySystem/UI_InventoryMenu.Find Slot by Name` _inventory (`self.Medallion 3`)))
  (if (`KismetTextLibrary.EqualEqual_TextText` "" (break `/Game/Game/Blueprints/InventorySystem/STRUCT_Item` _item))
    (`KismetSystemLibrary.PrintString` (`KismetTextLibrary.Conv_TextToString` (`self.Medallion 3`)))
    (else
      (`/Game/Game/Blueprints/InventorySystem/UI_InventoryMenu.Clear Slot by Name` _inventory (`self.Medallion 3`))
      (`SceneComponent.SetHiddenInGame` (`self.medal3`) false false)
      (return true))))

(fn `UserConstructionScript`
  (`parent.UserConstructionScript`))