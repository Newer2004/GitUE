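; Zombie enemy character that slaps Leon, reacts to hits and dies.
; While the attack flag is active, its trigger overlap applies randomly scaled slap damage to BP_Leon.
; Incoming damage drives the anim blueprint's hit reaction, notifies the AI controller and feeds the health component; death disables capsule collision and stops AI logic.
; A helper function switches max walk speed between walking and running.
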(event `self.Attack Trigger.OnComponentBeginOverlap`
  (params (OverlappedComponent :type "PrimitiveComponent Object Reference") (OtherActor :type "Actor Object Reference") (OtherComp :type "PrimitiveComponent Object Reference") (OtherBodyIndex :type Integer) (bFromSweep :type Boolean) (SweepResult :type "HitResult Structure (by ref)"))
  (if (`self.AttackTrigger Active`)
    (bind _asbp_leon (cast `/Game/Game/Leon/Blueprint/BP_Leon` OtherActor))
    (`GameplayStatics.ApplyDamage` _asbp_leon (* (`self.Slap Damage`) (`KismetMathLibrary.RandomFloatInRange` 0.7 1.0)) null self)))

(event `self.ReceiveAnyDamage`
  (params (Damage :type "Float (single-precision)") (DamageType :type "DamageType Object Reference") (InstigatedBy :type "Controller Object Reference") (DamageCauser :type "Actor Object Reference"))
  (bind _asabp_zombie (cast `/Game/Game/Blueprints/Enemies/Zombie/ABP_Zombie` (`SkeletalMeshComponent.GetAnimInstance` (`self.Mesh`))))
  (set `/Game/Game/Blueprints/Enemies/Zombie/ABP_Zombie.Hit Reaction Alpha` 1.0 _asabp_zombie)
  (bind _asai_zombie (cast `/Game/Game/Blueprints/Enemies/Zombie/AI_Zombie` (`AIBlueprintHelperLibrary.GetAIController` self)))
  (`/Game/Game/Blueprints/Enemies/Zombie/AI_Zombie.Got Hit` _asai_zombie)
  (set `self.Taking Damage` true)
  (bind _dead (`/Game/Game/Blueprints/HealthSystem/BP_HealthComponent.Hurt` (`self.BP_HealthComponent`) (`KismetMathLibrary.FTrunc` Damage)))
  (bind _output_get (set `self.Is Dead` _dead))
  (if _output_get
    (`PrimitiveComponent.SetCollisionEnabled` (`self.CapsuleComponent`) "NoCollision")
    (`BrainComponent.StopLogic` (`AIController.BrainComponent` (`AIBlueprintHelperLibrary.GetAIController` self)) "I am dead")))

(fn `Update Walk Speed`
  (params (`Is Running` :type Boolean))
  (set `CharacterMovementComponent.MaxWalkSpeed` (`KismetMathLibrary.SelectFloat` (`self.Run Speed`) (`self.Walk Speed`) `Is Running`) (`self.CharacterMovement`)))

(fn `UserConstructionScript`)