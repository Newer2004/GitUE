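; Shotgun weapon child Blueprint that adds a crosshair widget, pellet hit logic, and firing and reload feedback.
; Linetrace fires eight random cone traces from Leon's camera, spawning impact sparks and applying damage, with debug drawing left on.
; The damage select appears inverted: "Head" bone hits get base damage, while all others get the 1.5x multiplier.
; PlayFX triggers sound, muzzle flash and camera shake.
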(event `self.ReceiveBeginPlay`
  (`parent.ReceiveBeginPlay`)
  (bind _returnvalue (`|CreateWidget` "/Game/Game/Blueprints/Weapons/UI_Shotgun.UI_Shotgun_C"))
  (set `self.Crosshair UI` _returnvalue))

(fn `Get Linetrace Params`
  (returns (Start :type "Vector Structure") (End :type "Vector Structure"))
  (bind (_camera_transform_location _camera_transform_rotation) (`KismetMathLibrary.BreakTransform` (`/Game/Game/Leon/Blueprint/BP_Leon.Get Camera Transform` (`self.Leon ref`))))
  (return _camera_transform_location (+ _camera_transform_location (* (`KismetMathLibrary.RandomUnitVectorInConeInDegrees` (`KismetMathLibrary.GetForwardVector` _camera_transform_rotation) (`self.Spread Degrees`)) 9999999.0))))

(fn `Linetrace`
  (bind (_start _end) (`self.Get Linetrace Params`))
  (bind _damage (`self.Damage`))
  (for _ (range 1 9)
    (bind _outhit (`KismetSystemLibrary.LineTraceSingle` _start _end "TraceTypeQuery1" false (`|MakeArray` (`self.Leon ref`) :!type "Actor Object Reference") "ForDuration"))
    (`|ExecutionSequence`
      (:`then_0`
        (bind (_bblockinghit _binitialoverlap _time _distance _location _impactpoint _normal _impactnormal _physmat _hitactor _hitcomponent _hitbonename) (`GameplayStatics.BreakHitResult` _outhit))
        (`GameplayStatics.ApplyDamage` _hitactor (`KismetMathLibrary.SelectFloat` _damage (* _damage 1.5) (== _hitbonename "Head"))))
      (:`then_1`
        (`GameplayStatics.SpawnEmitterAtLocation` "/Game/MilitaryWeapDark/FX/P_Impact_Metal_Small_01.P_Impact_Metal_Small_01" _impactpoint (`KismetMathLibrary.MakeRotFromX` _impactnormal))))))

(fn `Play FX`
  (bind _camera_transform_location (`KismetMathLibrary.BreakTransform` (`/Game/Game/Leon/Blueprint/BP_Leon.Get Camera Transform` (`self.Leon ref`))))
  (`GameplayStatics.PlaySound2D` "/Game/MilitaryWeapDark/Sound/Shotgun/Wavs/ShotgunB_Fire02.ShotgunB_Fire02" 1.0 1.0 0.0 null null)
  (`ActorComponent.Activate` (`self.Muzzle Flash FX`) true)
  (`GameplayStatics.PlayWorldCameraShake` "/Game/Game/Blueprints/Weapons/CS_Shotgun.CS_Shotgun_C" _camera_transform_location 0.0 100.0))

(fn `Reload`
  (`parent.Reload`)
  (`GameplayStatics.PlaySound2D` "/Game/MilitaryWeapDark/Sound/Shotgun/Wavs/Shotgun_Reload02.Shotgun_Reload02" 1.0 1.0 0.0 null null))

(fn `UserConstructionScript`
  (`parent.UserConstructionScript`))