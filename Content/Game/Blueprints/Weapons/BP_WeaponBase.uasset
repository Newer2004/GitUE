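; Base weapon Blueprint for the player character BP_Leon, providing shared shooting, ammo and crosshair logic.
; Shoot runs Linetrace then PlayFX, both empty here, and does not itself consume ammo.
; Reload refills the clip from Leon's inventory reserve for the weapon type, with separate functions for reload checks and per-round consumption.
; Crosshair functions toggle the UI widget and scale it by spread percentage.
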(event `self.ReceiveBeginPlay`
  (bind _asbp_leon (cast `/Game/Game/Leon/Blueprint/BP_Leon` (`GameplayStatics.GetPlayerCharacter` 0)))
  (set `self.Leon ref` _asbp_leon))

(fn `Can Reload`
  (returns (`Can Reload` :type Boolean))
  (return (and (!= (`self.Current Ammo`) (`self.Clip Size`)) (!= (`self.Total Ammo`) 0))))

(fn `Consume Ammo`
  (returns (Success :type Boolean))
  (locals (`Cur Ammo` :type Integer))
  (if (> (`self.Current Ammo`) 0)
    (`/Engine/EditorBlueprintResources/StandardMacros.DecrementInt` (`self.Current Ammo`)
      (:`  `
        (return true)))
    (else
      (return false))))

(fn `Linetrace`)

(fn `Play FX`)

(fn `Reload`
  (locals (`Ammo To Add` :type Integer :default 0))
  (bind _output_get (set `local.Ammo To Add` (`KismetMathLibrary.Min` (- (`self.Clip Size`) (`self.Current Ammo`)) (`self.Total Ammo`))))
  (set `self.Current Ammo` (+ _output_get (`self.Current Ammo`)))
  (`/Game/Game/Blueprints/InventorySystem/UI_InventoryMenu.Remove Ammo` (`/Game/Game/Leon/Blueprint/BP_Leon.Inventory` (`self.Leon ref`)) (`local.Ammo To Add`) (`self.Weapon Type`)))

(fn `Shoot`
  (`self.Linetrace`)
  (`self.Play FX`))

(fn `Show Crosshair`
  (params (Show :type Boolean))
  (bind _crosshair_ui (`self.Crosshair UI`))
  (`/Engine/EditorBlueprintResources/StandardMacros.IsValid` (`self.Crosshair UI`)
    (:`Is Valid`
      (if Show
        (`UserWidget.AddToViewport` _crosshair_ui 0)
        (else
          (`Widget.RemoveFromParent` _crosshair_ui))))))

(fn `Total Ammo`
  (returns (`Total Ammo` :type Integer))
  (return (`/Game/Game/Blueprints/InventorySystem/UI_InventoryMenu.Total Ammo` (`/Game/Game/Leon/Blueprint/BP_Leon.Inventory` (`self.Leon ref`)) (`self.Weapon Type`))))

(fn `Update Crosshair Size`
  (params (`Spread Percent` :type "Float (double-precision)"))
  (bind _output_get (set `self.Current Spread Percent` `Spread Percent`))
  (`/Game/Game/Blueprints/Weapons/UI_CrosshairBase.Update Crosshair Size` (`self.Crosshair UI`) (* _output_get (`self.Max Spread Pixels`))))

(fn `UserConstructionScript`)