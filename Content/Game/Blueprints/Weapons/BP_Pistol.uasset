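; Pistol weapon Blueprint that extends a parent weapon with hitscan shooting, crosshair UI, effects and reload sound.
; Creates its crosshair widget on BeginPlay and plays fire sound, muzzle flash and camera shake in PlayFX.
; Linetrace fires from LeonRef's camera within a random cone scaled by current spread, applying damage with a headshot bonus and spawning metal impact particles.
; Debug trace drawing and bone-name printing remain enabled.
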(event `self.ReceiveBeginPlay`
  (`parent.ReceiveBeginPlay`)
  (bind _returnvalue (`|CreateWidget` "/Game/Game/Blueprints/Weapons/UI_Pistol.UI_Pistol_C"))
  (set `self.Crosshair UI` _returnvalue))

(fn `Get Linetrace Params`
  (returns (Start :type "Vector Structure") (End :type "Vector Structure"))
  (bind (_camera_transform_location _camera_transform_rotation) (`KismetMathLibrary.BreakTransform` (`/Game/Game/Leon/Blueprint/BP_Leon.Get Camera Transform` (`self.Leon ref`))))
  (return _camera_transform_location (+ _camera_transform_location (* (`KismetMathLibrary.RandomUnitVectorInConeInDegrees` (`KismetMathLibrary.GetForwardVector` _camera_transform_rotation) (* (`self.Max Spread Degrees`) (`self.Current Spread Percent`))) 9999999.0))))

(fn `Linetrace`
  (bind (_start _end) (`self.Get Linetrace Params`))
  (bind _damage (`self.Damage`))
  (bind _outhit (`KismetSystemLibrary.LineTraceSingle` _start _end "TraceTypeQuery3" false (`|MakeArray` (`self.Leon ref`) :!type "Actor Object Reference") "ForDuration"))
  (`|ExecutionSequence`
    (:`then_0`
      (bind (_bblockinghit _binitialoverlap _time _distance _location _impactpoint _normal _impactnormal _physmat _hitactor _hitcomponent _hitbonename) (`GameplayStatics.BreakHitResult` _outhit))
      (`KismetSystemLibrary.PrintString` (`KismetStringLibrary.Conv_NameToString` _hitbonename))
      (`GameplayStatics.ApplyDamage` _hitactor (`KismetMathLibrary.SelectFloat` (* _damage 1.5) _damage (== _hitbonename "Head"))))
    (:`then_1`
      (`GameplayStatics.SpawnEmitterAtLocation` "/Game/MilitaryWeapDark/FX/P_Impact_Metal_Small_01.P_Impact_Metal_Small_01" _impactpoint (`KismetMathLibrary.MakeRotFromX` _impactnormal)))))

(fn `Play FX`
  (bind _camera_transform_location (`KismetMathLibrary.BreakTransform` (`/Game/Game/Leon/Blueprint/BP_Leon.Get Camera Transform` (`self.Leon ref`))))
  (`GameplayStatics.PlaySound2D` "/Game/MilitaryWeapDark/Sound/Pistol/PistolB_Fire_Cue.PistolB_Fire_Cue" 1.0 1.0 0.0 null null)
  (`ActorComponent.Activate` (`self.Muzzle Flash FX`) true)
  (`GameplayStatics.PlayWorldCameraShake` "/Game/Game/Blueprints/Weapons/CS_Pistol.CS_Pistol_C" _camera_transform_location 0.0 100.0))

(fn `Reload`
  (`parent.Reload`)
  (`GameplayStatics.PlaySound2D` "/Game/MilitaryWeapDark/Sound/Pistol/Pistol_ReloadInsert_Cue.Pistol_ReloadInsert_Cue" 1.0 1.0 0.0 null null))

(fn `UserConstructionScript`
  (`parent.UserConstructionScript`))